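; Perspective puzzle actor that hides a target actor and projects its image onto scene surfaces until the player lines up with the viewpoint.
; On BeginPlay, scene captures render the target, and box traces over distance-sorted ProjectOnTo actors spawn M_Projection decals, masked by captures of nearer surfaces.
; Capsule overlap enables Tick, easing the player's position and view into alignment.
; Alignment confirmed after a delay reveals the target, unlocks prop physics and destroys this actor.
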(event `self.ReceiveBeginPlay`
  (bind _projection_target (`self.Projection Target`))
  (`self.Project Item`)
  (`self.SetActorHiddenInGame` _projection_target true)
  (`self.SetActorEnableCollision` _projection_target false))

(event `self.ReceiveTick`
  (params (DeltaSeconds :type "Float (single-precision)"))
  ;[1 1 1] Tick Event
  ;;[1 1 1] Center the player to the projection
  (`self.Player Near Position`)
  ;;[1 1 1] Check if player is in proper Position
  (if (`self.is Player in Position`)
    (`KismetSystemLibrary.Delay` 1.0)
    ;;[1 1 1] Check Player Position again
    (if (`self.is Player in Position`)
      (`self.Release the Actor`))))

(event `self.Capsule.OnComponentBeginOverlap`
  (params (OverlappedComponent :type "PrimitiveComponent Object Reference") (OtherActor :type "Actor Object Reference") (OtherComp :type "PrimitiveComponent Object Reference") (OtherBodyIndex :type Integer) (bFromSweep :type Boolean) (SweepResult :type "HitResult Structure (by ref)"))
  ;[1 1 1] Check if player near Projection and if so Enable Tick
  (bind _character (message `/Game/FirstPersonBP/Blueprints/Interactions/BPI_Character.Get Character` OtherActor))
  (`/Engine/EditorBlueprintResources/StandardMacros.IsValid` _character
    (:`Is Valid`
      (set `self.Player near` true)
      (set `self.Character` _character)
      (`self.SetActorTickEnabled` true))))

(event `self.Capsule.OnComponentEndOverlap`
  (params (OverlappedComponent :type "PrimitiveComponent Object Reference") (OtherActor :type "Actor Object Reference") (OtherComp :type "PrimitiveComponent Object Reference") (OtherBodyIndex :type Integer))
  ;[1 1 1] Check if player near Projection and if so Enable Tick
  (bind _character (message `/Game/FirstPersonBP/Blueprints/Interactions/BPI_Character.Get Character` OtherActor))
  (`/Engine/EditorBlueprintResources/StandardMacros.IsValid` _character
    (:`Is Valid`
      (set `self.Player near` false)
      (`self.SetActorTickEnabled` false))))

(event `Disable Char Movement`
  ;[1 1 1] Disable/Enable movement (Not USed)
)

(event `Enable Char Movemennt`
  ;[1 1 1] Disable/Enable movement (Not USed)
)

(fn `is Player in Position`
  (returns (Return :type Boolean))
  (bind _character (`self.Character`))
  (`self.Character`
    (:`then`
      (return (and (== (`self.K2_GetActorLocation`) (`self.K2_GetActorLocation` _character) :`ErrorTolerance` 3.0) (== (`Pawn.GetControlRotation` _character) (`SceneComponent.K2_GetComponentRotation` (`self.SceneCaptureComponent2D`)) :`ErrorTolerance` 2.0))))
    (:`else`)))

(fn `Player Near Position`
  (bind _character (`self.Character`))
  (bind (_returnvalue_x _returnvalue_y) (`KismetMathLibrary.BreakVector` (`SceneComponent.K2_GetComponentLocation` (`self.SceneCaptureComponent2D`))))
  (bind _returnvalue (`self.K2_GetActorLocation` _character))
  (if (`self.Player near`)
    (bind _character_2 (`self.Character`)
      (:`then`
        (bind _returnvalue_2 (`Pawn.GetController` _character_2))
        (`Controller.SetControlRotation` _returnvalue_2 (`KismetMathLibrary.RInterpTo` (`Controller.GetControlRotation` _returnvalue_2) (`SceneComponent.K2_GetComponentRotation` (`self.SceneCaptureComponent2D`)) (`GameplayStatics.GetWorldDeltaSeconds`) 2.0))
        (`self.K2_SetActorLocation` _character (`KismetMathLibrary.VInterpTo` _returnvalue (`KismetMathLibrary.MakeVector` _returnvalue_x _returnvalue_y (.z _returnvalue)) (`GameplayStatics.GetWorldDeltaSeconds`) 5.0) false false)
        (return))
      (:`else`))))

(fn `Project Item`
  (bind _scenecapturecomponent2d (`self.SceneCaptureComponent2D`))
  (bind _scenecapturecomponent2dmask (`self.SceneCaptureComponent2DMask`))
  (`SceneComponent.K2_SetWorldRotation` (`self.SceneCaptureComponent2D`) (`KismetMathLibrary.FindLookAtRotation` (`SceneComponent.K2_GetComponentLocation` (`self.SceneCaptureComponent2D`)) (`self.K2_GetActorLocation` (`self.Projection Target`))) false false)
  (`SceneComponent.K2_SetWorldRotation` (`self.SceneCaptureComponent2DMask`) (`KismetMathLibrary.FindLookAtRotation` (`SceneComponent.K2_GetComponentLocation` (`self.SceneCaptureComponent2D`)) (`self.K2_GetActorLocation` (`self.Projection Target`))) false false)
  (`KismetArrayLibrary.Array_Add` (`SceneCaptureComponent.ShowOnlyActors` (`self.SceneCaptureComponent2D`)) (`self.Projection Target`))
  (`KismetArrayLibrary.Array_Add` (`SceneCaptureComponent.ShowOnlyActors` (`self.SceneCaptureComponent2DMask`)) (`self.Projection Target`))
  (`|ExecutionSequence`
    (:`then_0`
      (bind _returnvalue (`KismetRenderingLibrary.CreateRenderTarget2D` 2048 2048))
      (set `SceneCaptureComponent2D.TextureTarget` _returnvalue _scenecapturecomponent2d)
      (`SceneCaptureComponent2D.CaptureScene` _scenecapturecomponent2d))
    (:`then_1`
      (bind _returnvalue_2 (`KismetRenderingLibrary.CreateRenderTarget2D` 2048 2048))
      (set `SceneCaptureComponent2D.TextureTarget` _returnvalue_2 _scenecapturecomponent2dmask)
      (`SceneCaptureComponent2D.CaptureScene` _scenecapturecomponent2dmask))
    (:`then_2`
      (`self.Sort by Distance`))
    (:`then_3`
      (`self.Projection Trace`))))

(fn `Projection Trace`
  (locals (`Ignore Actors` :type "Array of Actor Object Reference") (`Current Target` :type "Actor Object Reference") (`Show Only` :type "Array of Actor Object Reference") (Decal :type "DecalComponent Object Reference"))
  (bind (_returnvalue _returnvalue2 _outputpin _returnvalue3) (`self.Trace Input`))
  (bind (_returnvalue_2 _returnvalue2_2 _outputpin_2 _returnvalue3_2) (`self.Trace Input`))
  (bind _outhits (`KismetSystemLibrary.BoxTraceMulti` _returnvalue _returnvalue2 _outputpin _returnvalue3 "TraceTypeQuery1" false (`self.Project On To`)))
  (for _array_element _outhits
    (`KismetArrayLibrary.Array_AddUnique` (`local.Ignore Actors`) (`.HitActor` (`GameplayStatics.BreakHitResult` _array_element))))
  (for _array_element_2 (`self.Project On To`)
    (set `local.Current Target` _array_element_2)
    (bind _outhit (`KismetSystemLibrary.BoxTraceSingle` _returnvalue_2 _returnvalue2_2 _outputpin_2 _returnvalue3_2 "TraceTypeQuery1" false (`local.Ignore Actors`)))
    (`|ExecutionSequence`
      (:`then_0`
        (bind (_bblockinghit _binitialoverlap _time _distance _location _impactpoint _normal _impactnormal _physmat _hitactor _hitcomponent _hitbonename _hititem _elementindex _faceindex _tracestart _traceend) (`GameplayStatics.BreakHitResult` _outhit))
        (bind _asstatic_mesh_component (cast `StaticMeshComponent` _hitcomponent))
        (bind _returnvalue_3 (`self.GetTransform` (`ActorComponent.GetOwner` _asstatic_mesh_component)))
        (bind (_min _max) (`StaticMeshComponent.GetLocalBounds` _asstatic_mesh_component))
        (bind _returnvalue_4 (`AddComponent|NODE_AddDecalComponent-0` :`bManualAttachment` true :`RelativeTransform` (`KismetMathLibrary.MakeTransform` (+ (* (`KismetMathLibrary.Normal` (- _tracestart _traceend)) 5.1) (/ (+ (`KismetMathLibrary.TransformLocation` _returnvalue_3 _min) (`KismetMathLibrary.TransformLocation` _returnvalue_3 _max)) 2.0)) (`SceneComponent.K2_GetComponentRotation` _asstatic_mesh_component))))
        (bind _output_get (set `local.Decal` _returnvalue_4))
        (`SceneComponent.SetWorldScale3D` _output_get (+ (* _max (`SceneComponent.K2_GetComponentScale` _asstatic_mesh_component)) 5.0))
        (bind _returnvalue_5 (`KismetRenderingLibrary.CreateRenderTarget2D` 1024 1024))
        (bind _returnvalue_6 (`AddComponent|NODE_AddSceneCaptureComponent2D-0` :`RelativeTransform` (`SceneComponent.GetRelativeTransform` (`self.SceneCaptureComponent2D`))))
        (set `self.Scene Capture Depth` _returnvalue_6)
        (bind _output_get_2 (set `SceneCaptureComponent2D.TextureTarget` _returnvalue_5 _returnvalue_6))
        (`KismetArrayLibrary.Array_Append` (`SceneCaptureComponent.ShowOnlyActors` _returnvalue_6) (`local.Show Only`))
        (`SceneCaptureComponent2D.CaptureScene` _returnvalue_6)
        (bind _returnvalue_7 (`KismetMaterialLibrary.CreateDynamicMaterialInstance` "/Game/CustomContent/Projection/Material/M_Projection.M_Projection"))
        (`DecalComponent.SetDecalMaterial` (`local.Decal`) _returnvalue_7)
        (`self.Update Material Properties` _returnvalue_7 _output_get_2))
      (:`then_1`
        (`KismetArrayLibrary.Array_Add` (`local.Show Only`) (`local.Current Target`))
        (`KismetArrayLibrary.Array_Add` (`local.Ignore Actors`) (`local.Current Target`))))))

(fn `Release the Actor`
  (bind _projection_target (`self.Projection Target`))
  (`self.SetActorHiddenInGame` _projection_target false)
  (`self.SetActorEnableCollision` _projection_target true)
  (bind _actor (message `/Game/FirstPersonBP/Blueprints/Interactions/BPI_Prop_Object.Get Prop Actor` (`self.Projection Target`)))
  (`/Engine/EditorBlueprintResources/StandardMacros.IsValid` _actor
    (:`Is Valid`
      (set `/Game/CustomContent/Prop/BP_MasterProp.IsLocked` false _actor)
      (`PrimitiveComponent.SetSimulatePhysics` (`/Game/CustomContent/Prop/BP_MasterProp.Prop` _actor) true)
      (`self.Enable Char Movemennt`)
      (`self.K2_DestroyActor`))
    (:`Is Not Valid`
      (`self.Enable Char Movemennt`)
      (`self.K2_DestroyActor`))))

(fn `Sort by Distance`
  (locals (`Local index 1` :type Integer) (`Local Actor 1` :type "Actor Object Reference") (`Local index 2` :type Integer) (`Local Actor 2` :type "Actor Object Reference"))
  (for _index (range (+ (`KismetArrayLibrary.Array_LastIndex` (`self.Project On To`)) 1))
    (bind _output_get (set `local.Local index 1` _index))
    (set `local.Local Actor 1` (`|GetArrayItem` (`self.Project On To`) _output_get))
    (for _index_2 (range (`local.Local index 1`) (+ (`KismetArrayLibrary.Array_LastIndex` (`self.Project On To`)) 1))
      (bind _output_get_2 (set `local.Local index 2` _index_2))
      (set `local.Local Actor 2` (`|GetArrayItem` (`self.Project On To`) _output_get_2))
      (if (< (`self.GetDistanceTo` (`local.Local Actor 2`)) (`self.GetDistanceTo` (`local.Local Actor 1`)))
        (`KismetArrayLibrary.Array_Swap` (`self.Project On To`) (`local.Local index 1`) (`local.Local index 2`))))))

(fn `Trace Input`
  (returns (ReturnValue :type "Vector Structure") (ReturnValue2 :type "Vector Structure") (OutputPin :type "Vector Structure") (ReturnValue3 :type "Rotator Structure"))
  (bind _returnvalue (`self.K2_GetActorLocation`))
  (return _returnvalue (+ _returnvalue (* (`SceneComponent.GetForwardVector` (`self.SceneCaptureComponent2D`)) 5000.0)) (200.0 200.0 200.0) (`SceneComponent.K2_GetComponentRotation` (`self.SceneCaptureComponent2D`))))

(fn `Update Material Properties`
  (params (Mat :type "MaterialInstanceDynamic Object Reference") (Texture :type "TextureRenderTarget2D Object Reference"))
  (`MaterialInstanceDynamic.SetVectorParameterValue` Mat "Location" (`KismetMathLibrary.Conv_VectorToLinearColor` (`SceneComponent.K2_GetComponentLocation` (`self.SceneCaptureComponent2D`))))
  (`MaterialInstanceDynamic.SetVectorParameterValue` Mat "Right Vector" (`KismetMathLibrary.Conv_VectorToLinearColor` (`SceneComponent.GetRightVector` (`self.SceneCaptureComponent2D`))))
  (`MaterialInstanceDynamic.SetVectorParameterValue` Mat "Up Vector" (`KismetMathLibrary.Conv_VectorToLinearColor` (`SceneComponent.GetUpVector` (`self.SceneCaptureComponent2D`))))
  (`MaterialInstanceDynamic.SetVectorParameterValue` Mat "Forward Vector" (`KismetMathLibrary.Conv_VectorToLinearColor` (`SceneComponent.GetForwardVector` (`self.SceneCaptureComponent2D`))))
  (`MaterialInstanceDynamic.SetScalarParameterValue` Mat "Fov" (`SceneCaptureComponent2D.FOVAngle` (`self.SceneCaptureComponent2D`)))
  (`MaterialInstanceDynamic.SetTextureParameterValue` Mat "Projected Texture" (`SceneCaptureComponent2D.TextureTarget` (`self.SceneCaptureComponent2D`)))
  (`MaterialInstanceDynamic.SetTextureParameterValue` Mat "Projected Mask" Texture)
  (`MaterialInstanceDynamic.SetTextureParameterValue` Mat "Actor Mask" (`SceneCaptureComponent2D.TextureTarget` (`self.SceneCaptureComponent2DMask`))))

(fn `UserConstructionScript`
  (set `PrimitiveComponent.bGenerateOverlapEvents` (`self.Should Generate Event`) (`self.Capsule`)))
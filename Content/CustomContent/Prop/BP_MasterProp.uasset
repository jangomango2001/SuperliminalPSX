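; Base physics prop that can be picked up and dropped, unless flagged as locked.
; PickUp attaches the mesh to a given component with physics and collision off, and Drop detaches it and re-enables both.
; Locked props disable physics on BeginPlay and refuse both actions.
; ResetRotation eases the mesh one step per call toward upright while keeping yaw, and getters expose the actor and mesh.
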(event `self.ReceiveBeginPlay`
  (if (`self.IsLocked`)
    (`PrimitiveComponent.SetSimulatePhysics` (`self.Prop`) false)))

(event `Reset Rotation`
  (bind _prop (`self.Prop`))
  (bind _returnvalue (`SceneComponent.K2_GetComponentRotation` _prop))
  ;[1 1 1] Pickup Rotation reset
  (`SceneComponent.K2_SetWorldRotation` _prop (`KismetMathLibrary.RInterpTo` _returnvalue (`KismetMathLibrary.MakeRotator` 0.0 0.0 (.yaw _returnvalue)) (`GameplayStatics.GetWorldDeltaSeconds`) 10.0) false false))

(fn `Drop`
  (returns (`Picked Up?` :type Boolean))
  (if (`self.IsLocked`)
    (return false)
    (else
      (`SceneComponent.K2_DetachFromComponent` (`self.Prop`) "KeepWorld" "KeepWorld" "KeepWorld" true)
      (`PrimitiveComponent.SetCollisionEnabled` (`self.Prop`) "QueryAndPhysics")
      (`PrimitiveComponent.SetSimulatePhysics` (`self.Prop`) true)
      (set `self.IsHeld` false)
      (return false))))

(fn `Get Prop Actor`
  (returns (Actor :type "/Game/CustomContent/Prop/BP_MasterProp Object Reference"))
  (return self))

(fn `Get Prop Mesh`
  (returns (Prop :type "StaticMeshComponent Object Reference"))
  (return (`self.Prop`)))

(fn `PickUp`
  (params (`Parent Comp` :type "SceneComponent Object Reference"))
  (returns (`Picked Up?` :type Boolean))
  (bind _prop (`self.Prop`))
  (if (`self.IsLocked`)
    (return false)
    (else
      (`SceneComponent.K2_AttachToComponent` (`self.Prop`) `Parent Comp` "None" "KeepWorld" "KeepWorld" "KeepWorld" true)
      (`PrimitiveComponent.SetSimulatePhysics` _prop false)
      (`PrimitiveComponent.SetCollisionEnabled` _prop "NoCollision")
      (set `self.IsHeld` true)
      (return true))))

(fn `UserConstructionScript`)
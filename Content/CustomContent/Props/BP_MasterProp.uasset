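; BP_MasterProp is a prop actor, apparently meant as a base class, that can be picked up and dropped.
; PickUp attaches the Prop mesh to a given component with physics and collision off; Drop detaches it and restores both, keeping world transform.
; Both refuse when IsLocked, return success as a boolean, and set IsHeld to true, even on Drop.
; Getters expose the actor and mesh, and the event graph is empty.
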(fn `Drop`
  (returns (`Picked Up?` :type Boolean))
  (if (`self.IsLocked`)
    (return false)
    (else
      (`SceneComponent.K2_DetachFromComponent` (`self.Prop`) "KeepWorld" "KeepWorld" "KeepWorld" true)
      (`PrimitiveComponent.SetCollisionEnabled` (`self.Prop`) "QueryAndPhysics")
      (`PrimitiveComponent.SetSimulatePhysics` (`self.Prop`) true)
      (set `self.IsHeld` true)
      (return true))))

(fn `Get Prop Actor`
  (returns (Actor :type "/Game/CustomContent/Props/BP_MasterProp Object Reference"))
  (return self))

(fn `Get Prop Mesh`
  (returns (Prop :type "StaticMeshComponent Object Reference"))
  (return (`self.Prop`)))

(fn `PickUp`
  (params (`Parent Comp` :type "SceneComponent Object Reference"))
  (returns (`Picked Up?` :type Boolean))
  (bind _prop (`self.Prop`))
  (if (`self.IsLocked`)
    (return false)
    (else
      (`SceneComponent.K2_AttachToComponent` (`self.Prop`) `Parent Comp` "None" "KeepWorld" "KeepWorld" "KeepWorld" true)
      (`PrimitiveComponent.SetSimulatePhysics` _prop false)
      (`PrimitiveComponent.SetCollisionEnabled` _prop "NoCollision")
      (set `self.IsHeld` true)
      (return true))))

(fn `UserConstructionScript`)
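; Master physics prop for a Superliminal-style game that the player can highlight, pick up and drop unless locked.
; Duplicator props instead spawn a smaller copy at a player box-trace location, registering every copy with the original parent.
; Resetting duplicates lerps the copies back into that parent via a timeline, then destroys them.
; Throttled, speed-checked impacts play sounds scaled by prop size, with camera shake for large props.
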(event `self.ReceiveBeginPlay`
  (if (`self.IsLocked`)
    (`PrimitiveComponent.SetSimulatePhysics` (`self.Prop`) false)))

(event `Reset Rotation`
  (bind _prop (`self.Prop`))
  (bind _returnvalue (`SceneComponent.K2_GetComponentRotation` _prop))
  ;[1 1 1] Pickup Rotation reset
  (`SceneComponent.K2_SetWorldRotation` _prop (`KismetMathLibrary.RInterpTo` _returnvalue (`KismetMathLibrary.MakeRotator` 0.0 0.0 (.yaw _returnvalue)) (`GameplayStatics.GetWorldDeltaSeconds`) 10.0) false false))

(event `Highlight Object`
  (params (`Highlight?` :type Boolean))
  (bind _prop (`self.Prop`))
  ;[1 1 1] Highlight Object
  (if (not (`self.IsLocked`))
    (if `Highlight?`
      (`PrimitiveComponent.SetRenderCustomDepth` _prop true)
      (else
        (`PrimitiveComponent.SetRenderCustomDepth` _prop false)))))

(event `self.Prop.OnComponentHit`
  (params (HitComponent :type "PrimitiveComponent Object Reference") (OtherActor :type "Actor Object Reference") (OtherComp :type "PrimitiveComponent Object Reference") (NormalImpulse :type "Vector Structure") (Hit :type "HitResult Structure (by ref)"))
  (bind _prop (`self.Prop`))
  (bind _prop_2 (`self.Prop`))
  (bind _returnvalue (`KismetMathLibrary.VSize` (`SceneComponent.RelativeScale3D` _prop_2)))
  (bind _returnvalue_2 (`KismetMathLibrary.VSize` (`SceneComponent.RelativeScale3D` (`self.Prop`))))
  ;[1 1 1] Generic Hit Sound
  (if (`SceneComponent.IsSimulatingPhysics` (`self.Prop`) "None")
    (if (>= (* (`PrimitiveComponent.GetMass` _prop) (`KismetMathLibrary.VSize` (`SceneComponent.GetComponentVelocity` _prop))) 10000.0)
      (`|ExecutionSequence` :!label _label
        (:`then_0`
          (`/Engine/EditorBlueprintResources/StandardMacros.DoOnce` false :!label _label_2
            (:`Completed`
              (bind _returnvalue_3 (`GameplayStatics.SpawnSoundAtLocation` "/Game/Superliminal/Audio/Hit_Sounds/HitSound.HitSound" (`.Location` (`GameplayStatics.BreakHitResult` Hit)) (struct) (`KismetMathLibrary.MapRangeClamped` _returnvalue_2 5.0 0.2 5.0 0.98) (`KismetMathLibrary.MapRangeClamped` _returnvalue_2 0.2 5.0 1.1 0.7) 0.0 null null))
              (`/Engine/EditorBlueprintResources/StandardMacros.IsValid` _returnvalue_3 ; Sometimes the return value is NULL
                (:`Is Valid`
                  (`AudioComponent.SetIntParameter` _returnvalue_3 "Power" (`KismetMathLibrary.Round` (`KismetMathLibrary.MapRangeClamped` _returnvalue_2 0.1 5.0 0.0 5.0)))
                  (if (>= _returnvalue 1.5)
                    (`GameplayStatics.PlayWorldCameraShake` "/Game/Superliminal/Screen-Shake/Camera-Shake.Camera-Shake_C" (`SceneComponent.K2_GetComponentLocation` _prop_2) 10.0 (* _returnvalue (`KismetMathLibrary.VSize` (`SceneComponent.GetComponentVelocity` _prop_2)) 0.35))))))))
        (:`then_1`
          (`KismetSystemLibrary.Delay` (`KismetMathLibrary.RandomFloatInRange` 0.5 1.2))
          (goto _label_2 :!via `Reset`))))
    (else
      (goto _label))))

(event `Lerp Back to Parent`
  (bind _prop (`self.Prop`))
  ;[1 1 1] Lerp Transform Back & Destroy Actors
  (`PrimitiveComponent.SetSimulatePhysics` _prop false)
  (`PrimitiveComponent.SetCollisionEnabled` _prop "NoCollision")
  (bind (_direction _alpha) (`Timeline|Timeline_0` :!via `PlayFromStart`)
    (:`Update`
      (`SceneComponent.K2_SetWorldTransform` (`self.Prop`) (`KismetMathLibrary.TLerp` (`SceneComponent.K2_GetComponentToWorld` (`self.Prop`)) (`SceneComponent.K2_GetComponentToWorld` (`/Game/Superliminal/Prop/BP_MasterProp.Prop` (`self.Parent ref`))) _alpha) false false))
    (:`Finished`
      (`KismetArrayLibrary.Array_RemoveItem` (`/Game/Superliminal/Prop/BP_MasterProp.Spawned Children` (`self.Parent ref`)) self)
      (`self.K2_DestroyActor`))))

(event `Destroy all Children`
  ;[1 1 1] Lerp Transform Back & Destroy Actors
  (bind _character (message `/Game/Superliminal/Character/Blueprints/Interactions/BPI_Character.Get Character` (`GameplayStatics.GetPlayerCharacter` 0)))
  (`/Game/Superliminal/Character/Blueprints/My_Character.Pop Sound Effect` _character (`self.Prop`) false)
  (for _array_element (`self.Spawned Children`)
    (`self.Lerp Back to Parent` _array_element)))

(fn `Drop`
  (returns (`Picked Up?` :type Boolean))
  (if (`self.IsLocked`)
    (return false)
    (else
      (`SceneComponent.K2_DetachFromComponent` (`self.Prop`) "KeepWorld" "KeepWorld" "KeepWorld" true)
      (`PrimitiveComponent.SetCollisionEnabled` (`self.Prop`) "QueryAndPhysics")
      (`PrimitiveComponent.SetSimulatePhysics` (`self.Prop`) true)
      (`self.Highlight Object` false)
      (set `self.IsHeld` false)
      (return false))))

(fn `Duplicate`
  (bind (_origin _boxextent) (`KismetSystemLibrary.GetComponentBounds` (`self.Prop`)))
  (bind _character (message `/Game/Superliminal/Character/Blueprints/Interactions/BPI_Character.Get Character` (`GameplayStatics.GetPlayerCharacter` 0)))
  (`/Game/Superliminal/Character/Blueprints/My_Character.Pop Sound Effect` _character (`self.Prop`) true)
  (bind _location (`MyCharacter_Class.BoxTrace` _character (`self.Prop`) _boxextent (`KismetMathLibrary.Vector_Distance` (0.0 0.0 0.0) _boxextent) 3 "TraceTypeQuery1" (`|MakeArray` _character self :!type "Actor Object Reference")))
  (bind (_returnvalue_roll _returnvalue_pitch _returnvalue_yaw) (`KismetMathLibrary.BreakRotator` (`KismetMathLibrary.FindLookAtRotation` _location (`self.K2_GetActorLocation` _character))))
  (bind _returnvalue (`|SpawnActorFromClass` (`GameplayStatics.GetObjectClass` self) (`KismetMathLibrary.MakeTransform` _location (`KismetMathLibrary.MakeRotator` 0.0 0.0 _returnvalue_yaw) (/ (`SceneComponent.K2_GetComponentScale` (`self.Prop`)) 1.25)) "AdjustIfPossibleButAlwaysSpawn" "OverrideRootScale" null false null))
  (`PrimitiveComponent.SetSimulatePhysics` (`/Game/Superliminal/Prop/BP_MasterProp.Prop` _returnvalue) (`SceneComponent.IsSimulatingPhysics` (`self.Prop`) "None"))
  (set `/Game/Superliminal/Prop/BP_MasterProp.Parent ref` (select `bool` (`self.Is Child`) :`false` self :`true` (`self.Parent ref`) :!type "/Game/Superliminal/Prop/BP_MasterProp Object Reference") _returnvalue)
  (set `/Game/Superliminal/Prop/BP_MasterProp.Is Child` true _returnvalue)
  (set `/Game/Superliminal/Prop/BP_MasterProp.Is Duplicating Actor` true _returnvalue)
  (`KismetArrayLibrary.Array_Add` (select `bool` (`self.Is Child`) :`false` (`self.Spawned Children`) :`true` (`/Game/Superliminal/Prop/BP_MasterProp.Spawned Children` (`self.Parent ref`))) _returnvalue))

(fn `Get Prop Actor`
  (returns (Actor :type "/Game/Superliminal/Prop/BP_MasterProp Object Reference"))
  (return self))

(fn `Get Prop Mesh`
  (returns (Prop :type "StaticMeshComponent Object Reference"))
  (return (`self.Prop`)))

(fn `PickUp`
  (params (`Parent Comp` :type "SceneComponent Object Reference"))
  (returns (`Picked Up?` :type Boolean))
  (bind _prop (`self.Prop`))
  (if (`self.IsLocked`)
    (return false)
    (elif (not (`self.Is Duplicating Actor`))
      (`SceneComponent.K2_AttachToComponent` (`self.Prop`) `Parent Comp` "None" "KeepWorld" "KeepWorld" "KeepWorld" true)
      (`PrimitiveComponent.SetSimulatePhysics` _prop false)
      (`PrimitiveComponent.SetCollisionEnabled` _prop "NoCollision")
      (set `self.IsHeld` true)
      (return true)
      (else
        (`self.Duplicate`)
        (return false)))))

(fn `Reset Duplicates`
  (if (`self.Is Child`)
    (`self.Destroy all Children` (`self.Parent ref`))
    (else
      (`self.Destroy all Children`))))

(fn `Reset to Initial location`
  (`SceneComponent.K2_SetWorldTransform` (`self.Prop`) (`self.Initial Transformation`) false false))

(fn `UserConstructionScript`
  (set `self.Initial Transformation` (`SceneComponent.K2_GetComponentToWorld` (`self.Prop`))))
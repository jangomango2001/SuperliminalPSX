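; BP_End_Level is an end-of-level trigger that hands the player's exit from a level over to the game instance.
; When the character enters its box, it runs once to stop movement and disable input.
; It then passes LevelToLoad to the game instance, starts the fade widget and saves newest and unlocked levels.
; Its direct LoadLevel call is unconnected, so this Blueprint does not load the level itself.
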(event `self.Box.OnComponentBeginOverlap`
  (params (OverlappedComponent :type "PrimitiveComponent Object Reference") (OtherActor :type "Actor Object Reference") (OtherComp :type "PrimitiveComponent Object Reference") (OtherBodyIndex :type Integer) (bFromSweep :type Boolean) (SweepResult :type "HitResult Structure (by ref)"))
  (bind _character (message `/Game/Superliminal/Character/Blueprints/Interactions/BPI_Character.Get Character` OtherActor))
  (`/Engine/EditorBlueprintResources/StandardMacros.IsValid` _character
    (:`Is Valid`
      (bind _my_game_instance_ref (message `/Game/Superliminal/BPI_GameInstance.Get Game instance` (`GameplayStatics.GetGameInstance`)))
      (`/Engine/EditorBlueprintResources/StandardMacros.IsValid` _my_game_instance_ref
        (:`Is Valid`
          (`/Engine/EditorBlueprintResources/StandardMacros.DoOnce` false
            (:`Completed`
              (`self.DisableInput` _character (cast `PlayerController` (`Pawn.GetController` _character) :!pure true))
              (`MovementComponent.StopMovementImmediately` (`Character.CharacterMovement` _character))
              (set `/Game/Superliminal/MygameInstance.New Level Name` (`self.Level to Load`) _my_game_instance_ref)
              (`/Game/Superliminal/MygameInstance.Fade In Widget` _my_game_instance_ref)
              (`/Game/Superliminal/MygameInstance.Save Newest Level` _my_game_instance_ref)
              (`/Game/Superliminal/MygameInstance.Save unlocked Levels` _my_game_instance_ref))))
        (:`Is Not Valid`
          (`KismetSystemLibrary.PrintString` "BP_End_Level:: Game Instance Not Found" true true (struct :`R` 1.0 :`A` 1.0)))))
    (:`Is Not Valid`
      (`KismetSystemLibrary.PrintString` "BP_End_Level:: Char didn't enter" true true (struct :`R` 1.0 :`A` 1.0)))))

(fn `UserConstructionScript`)
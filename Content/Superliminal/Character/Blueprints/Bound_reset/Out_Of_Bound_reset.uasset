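; Out-of-bounds volume that sends props and the player back when they enter its box.
; On overlap, props reset to their initial location, while characters teleport to the reset point at the stored index.
; The construction script gives each reset point in its array a reference back to this volume.
; FindPoint sets that index from a given reset point actor, though nothing in this graph calls it.
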(event `self.Box.OnComponentBeginOverlap`
  (params (OverlappedComponent :type "PrimitiveComponent Object Reference") (OtherActor :type "Actor Object Reference") (OtherComp :type "PrimitiveComponent Object Reference") (OtherBodyIndex :type Integer) (bFromSweep :type Boolean) (SweepResult :type "HitResult Structure (by ref)"))
  (bind _actor (message `/Game/Superliminal/Character/Blueprints/Interactions/BPI_Prop_Object.Get Prop Actor` OtherActor))
  (`/Engine/EditorBlueprintResources/StandardMacros.IsValid` _actor
    (:`Is Valid`
      (`/Game/Superliminal/Prop/BP_MasterProp.Reset to Initial location` _actor))
    (:`Is Not Valid`
      (bind _character (message `/Game/Superliminal/Character/Blueprints/Interactions/BPI_Character.Get Character` OtherActor))
      (`/Engine/EditorBlueprintResources/StandardMacros.IsValid` _character
        (:`Is Valid`
          (`self.Teleport Player Back` _character))))))

(fn `Find Point`
  (params (Actor :type "/Game/Superliminal/Character/Blueprints/Bound_reset/Spawn-Points Object Reference"))
  (set `self.Point` (`KismetArrayLibrary.Array_Find` (`self.Reset Points`) Actor)))

(fn `Teleport Player Back`
  (params (Character :type "/Game/Superliminal/Character/Blueprints/My_Character Object Reference"))
  (locals (`Selected Actor local` :type "/Game/Superliminal/Character/Blueprints/Bound_reset/Spawn-Points Object Reference"))
  (bind _output_get (set `local.Selected Actor local` (`|GetArrayItem` (`self.Reset Points`) (`self.Point`))))
  (`/Engine/EditorBlueprintResources/StandardMacros.IsValid` _output_get
    (:`Is Valid`
      (`self.K2_SetActorLocation` Character (`self.K2_GetActorLocation` (`local.Selected Actor local`)) false true))))

(fn `UserConstructionScript`
  (for _array_element (`self.Reset Points`)
    (set `/Game/Superliminal/Character/Blueprints/Bound_reset/Spawn-Points.Out of Bound Volume Ref` self _array_element)))
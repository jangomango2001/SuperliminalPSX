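; Rotating lighthouse beacon for the Coldharbour Seaside demo environment, with a configurable spotlight.
; The Construction Script applies intensity, attenuation radius and inner and outer cone angle variables to the SpotLight.
; Tick adds a fixed relative rotation to the scene root without scaling by delta time, so spin speed depends on frame rate.
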(event `self.ReceiveTick`
  (params (DeltaSeconds :type "Float (single-precision)"))
  (`SceneComponent.K2_AddRelativeRotation` (`self.DefaultSceneRoot`) (struct :`Yaw` 1.0) false false))

(fn `UserConstructionScript`
  (bind _spotlight (`self.SpotLight`))
  (bind _spotlight_2 (`self.SpotLight`))
  (`LightComponent.SetIntensity` _spotlight (`self.New Intensity`))
  (`LocalLightComponent.SetAttenuationRadius` _spotlight (`self.New Radius`))
  (`SpotLightComponent.SetInnerConeAngle` _spotlight_2 (`self.New Inner Cone Angle`))
  (`SpotLightComponent.SetOuterConeAngle` _spotlight_2 (`self.New Outer Cone Angle`)))